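; Team Deathmatch game mode that runs the timed match and reports each side's outcome from the winning team.
; On BeginPlay it reads player cap and bot settings, updates the online session, toggles AI spawners and caches team starts.
; Spawning picks a random side start free of pawns via box overlap, optionally falling back to occupied ones.
; Tick starts and ends the match; any TriggerVolume overlap moves operators to world origin.
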(event `self.ReceiveBeginPlay`
  (`self.Load Mission Settings`)
  (`self.UpdateSession`
    (:`Out`
      (`self.Init Bots`)
      (bind _outactors (`GameplayStatics.GetAllActorsOfClass` "/TeamDeathmatch/TDM/Blueprints/PlayerStart/B_TDM_Blue_PlayerStart.B_TDM_Blue_PlayerStart_C"))
      (set `self.bluePlayerStart` _outactors)
      (bind _outactors_2 (`GameplayStatics.GetAllActorsOfClass` "/TeamDeathmatch/TDM/Blueprints/PlayerStart/B_TDM_Op_PlayerStart.B_TDM_Op_PlayerStart_C"))
      (set `self.opPlayerStart` _outactors_2)
      (bind _outactors_3 (`GameplayStatics.GetAllActorsOfClass` "/Script/Engine.TriggerVolume"))
      (for _array_element _outactors_3
        (add `self.OnActorBeginOverlap` _array_element (delegate `OnActorBeginOverlap_Event_0`))))))

(event `OnActorBeginOverlap_Event_0` :!signature `self.OnActorBeginOverlap`
  (params (OverlappedActor :type "Actor Object Reference") (OtherActor :type "Actor Object Reference"))
  (bind _asb_operator (cast `/Game/Blueprints/Character/Blufor/B_Operator` OtherActor))
  (`SceneComponent.K2_SetWorldLocation` (`Actor.RootComponent` _asb_operator) (0.0 0.0 0.0) false false))

(event `self.ReceiveTick`
  (params (DeltaSeconds :type "Float (single-precision)"))
  (if (`self.debugDraw`)
    ;[1 1 1] Debug
    (for _ (`self.bluePlayerStart`)
      (`KismetSystemLibrary.DrawDebugBox` (`self.K2_GetActorLocation`) (`self.spawnBoxSize`) (struct :`R` 1.0 :`G` 0.070607 :`A` 1.0))))
  (`KismetSystemLibrary.Delay` 0.6)
  (if (`GameStateBase.HasMatchStarted` (`GameplayFunctionLibrary.GetGameState`))
    (if (== (`MatchGameState.GetMatchTimeLeft` (`GameplayFunctionLibrary.GetMatchState`)) 0.0)
      (`self.EndMatch`))
    (else
      (`self.StartMatch`))))

(fn `Check Player Area`
  (params (AreaPosition :type "Vector Structure") (AreaSize :type "Vector Structure"))
  (returns (`Contains Players` :type Boolean))
  (bind _outactors (`KismetSystemLibrary.BoxOverlapActors` AreaPosition AreaSize (`|MakeArray` "ObjectTypeQuery3" :!type "EObjectTypeQuery Enum")))
  (return (> (`KismetArrayLibrary.Array_Length` _outactors) 0)))

(fn `FindPlayerStart`
  (params (Player :type "Controller Object Reference") (IncomingName :type String))
  (returns (ReturnValue :type "Actor Object Reference"))
  (bind _asb_soldier_player_controller (cast `/Game/Blueprints/Game/Controllers/Player/B_SoldierPlayerController` Player))
  (switch `EPlayableSide` (`SoldierPlayerController.GetPlayerSide` _asb_soldier_player_controller)
    (:`Side_None`
      _)
    (:`Side_Bluefor`
      (bind _bestplayerstart (`self.SearchBestPlayerStart` (`self.bluePlayerStart`)))
      (return _bestplayerstart))
    (:`Side_Opfor`
      (bind _bestplayerstart_2 (`self.SearchBestPlayerStart` (`self.opPlayerStart`)))
      (return _bestplayerstart_2))
    (:`Side_Civ`
      _)
    (:`Side_AlwaysEnemy`
      _))
  (bind _returnvalue (`parent.FindPlayerStart` Player ""))
  (return _returnvalue))

(fn `GetSideOutcomeType`
  (params (InSide :type "EPlayableSide Enum" :default "Side_None"))
  (returns (ReturnValue :type "EGameModeOutcomeType Enum"))
  (bind _asb_tdm_game_state (cast `/TeamDeathmatch/TDM/Blueprints/GameState/B_TDM_GameState` (`GameplayStatics.GetGameState`)))
  (bind _winning_team (`/TeamDeathmatch/TDM/Blueprints/GameState/B_TDM_GameState.GetWinningTeam` _asb_tdm_game_state))
  (if (`|EnumEquality` _winning_team "Side_None")
    (return "GMOT_Draw")
    (elif (`|EnumEquality` _winning_team InSide)
      (return "GMOT_Victory")
      (else
        (return "GMOT_Defeat")))))

(fn `Init Bots`
  (bind _outactors (`GameplayStatics.GetAllActorsOfClass` "/Script/Thunder2305.AISpawnerActor"))
  (for _array_element _outactors
    (if (`self.settingsEnableBots`)
      (`AISpawnerActor.EnableSpawner` _array_element true)
      (else
        (`AISpawnerActor.DisableSpawner` _array_element)))))

(fn `Load Mission Settings`
  (locals (initEnableBot :type Boolean))
  (`|ExecutionSequence`
    (:`then_0`
      (bind (_boutsettingfound _outmissionsetting) (`GameplayFunctionLibrary.GetMissionSettingById` "SuddenDeathMode"))
      (if _boutsettingfound
        (set `self.maxPlayers` (`.ValueInt` (break `MissionSetting` _outmissionsetting)))))
    (:`then_1`
      (bind (_boutsettingfound_2 _outmissionsetting_2) (`GameplayFunctionLibrary.GetMissionSettingById` "LoneWolf"))
      (if _boutsettingfound_2
        (bind (_id _displayname _tooltip _type _bshowinmp _bactive _unit _defaultvaluefloat _minvaluefloat _maxvaluefloat _defaultvalueint _minvalueint _maxvalueint _defaultvaluebool _defaultvalueweaponclass _valuefloat _valueint _valuebool) (break `MissionSetting` _outmissionsetting_2))
        (set `self.settingsEnableBots` (`KismetMathLibrary.Conv_IntToBool` _valuebool))
        ;[1 1 1] Testing
        (`KismetSystemLibrary.PrintString` (`KismetStringLibrary.Concat_StrStr` (`|GetEnumeratorNameAsString` _id) (`KismetTextLibrary.Conv_TextToString` _displayname) (`KismetTextLibrary.Conv_TextToString` _tooltip) (`|GetEnumeratorNameAsString` _type) (`KismetStringLibrary.Conv_BoolToString` _bshowinmp) (`KismetStringLibrary.Conv_BoolToString` _bactive) (`KismetStringLibrary.Conv_DoubleToString` _defaultvaluefloat) (`KismetStringLibrary.Conv_DoubleToString` _minvaluefloat) (`KismetStringLibrary.Conv_DoubleToString` _maxvaluefloat) (`KismetStringLibrary.Conv_IntToString` _defaultvalueint) (`KismetStringLibrary.Conv_IntToString` _minvalueint) (`KismetStringLibrary.Conv_IntToString` _maxvalueint) (`KismetStringLibrary.Conv_BoolToString` _defaultvaluebool) (`KismetStringLibrary.Conv_DoubleToString` _valuefloat) (`KismetStringLibrary.Conv_IntToString` _valueint) (`KismetStringLibrary.Conv_IntToString` _valuebool)))))))

(fn `SearchBestPlayerStart`
  (params (PlayerStartList :type "Array of PlayerStart Object Reference"))
  (returns (bestPlayerStart :type "PlayerStart Object Reference"))
  (locals (tempPlayerStartArray :type "Array of PlayerStart Object Reference"))
  (bind _tempplayerstartarray (`local.tempPlayerStartArray`))
  ;[1 1 1] Spawn player if there is at least 1 spawn actor
  (if (> (`KismetArrayLibrary.Array_Length` PlayerStartList) 0)
    (for _array_element PlayerStartList
      ;[1 1 1] Add all possible free slots
      (bind _contains_players (`self.Check Player Area` (`self.K2_GetActorLocation` _array_element) (`self.spawnBoxSize`)))
      (if (not _contains_players)
        (`KismetArrayLibrary.Array_Add` (`local.tempPlayerStartArray`) _array_element)))
    (if (> (`KismetArrayLibrary.Array_Length` _tempplayerstartarray) 0)
      (return (`/Game/Blueprints/Game/B_BlueprintGameplayMacros.GetRandomArrayElement` _tempplayerstartarray))
      (elif (not (`self.AvailableSpawnOnly`))
        (return (`/Game/Blueprints/Game/B_BlueprintGameplayMacros.GetRandomArrayElement` PlayerStartList))))))

(fn `UserConstructionScript`)
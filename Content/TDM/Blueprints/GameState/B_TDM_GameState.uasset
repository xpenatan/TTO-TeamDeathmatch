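; Team Deathmatch game state that keeps the Bluefor and Opfor kill scores and reports the winning side.
; On authority, BeginPlay binds to player-killed and AI-killed events, each crediting a kill to the side opposing the dead soldier, regardless of who the killer is.
; GetWinningTeam compares the two totals and returns None on a tie.
; Per-player kill summing is deprecated and disconnected, and AddPlayerKills and AddEnemyKills do nothing.
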(event `self.ReceiveBeginPlay`
  (`/Engine/EditorBlueprintResources/ActorMacros.Switch Has Authority`
    (:`Authority`
      (add `MatchGameState.OnAIKilled` (delegate `OnAIKilled_Event_0`))
      (add `MatchGameState.OnPlayerKilled` (delegate `OnPlayerKilled_Event_0`)))))

(event `OnPlayerKilled_Event_0`
  (params (InDead :type "PlayerState Object Reference") (InKiller :type "PlayerState Object Reference") (DeadData :type "ReplicatedDead Structure (by ref)"))
  (bind _asb_base_soldier (cast `/Game/Blueprints/Character/B_BaseSoldier` DeadData_DamageReceiver))
  (switch `EPlayableSide` (`HostageCharacter.GetSide` _asb_base_soldier)
    (:`Side_Bluefor`
      (`self.Add Side Kill` "Side_Opfor"))
    (:`Side_Opfor`
      (`self.Add Side Kill` "Side_Bluefor"))))

(event `OnAIKilled_Event_0`
  (params (InDead :type "Pawn Object Reference") (InKiller :type "Actor Object Reference"))
  ;[1 1 1] When player killed AI or AI Killed AI
  (bind _asb_base_soldier (cast `/Game/Blueprints/Character/B_BaseSoldier` InDead))
  (switch `EPlayableSide` (`HostageCharacter.GetSide` _asb_base_soldier)
    (:`Side_Bluefor`
      (`self.Add Side Kill` "Side_Opfor"))
    (:`Side_Opfor`
      (`self.Add Side Kill` "Side_Bluefor"))))

(event `self.ReceiveTick`
  (params (DeltaSeconds :type "Float (single-precision)")))

(fn `Add Side Kill`
  (params (Side :type "EPlayableSide Enum" :default "Side_None"))
  (switch `EPlayableSide` Side
    (:`Side_Bluefor`
      (set `self.BlueFor` (+ (`self.BlueFor`) 1)))
    (:`Side_Opfor`
      (set `self.OpFor` (+ (`self.OpFor`) 1)))))

(fn `AddEnemyKills`)

(fn `AddPlayerKills`
  (params (KillerPlayerState :type "/TeamDeathmatch/TDM/Blueprints/PlayerState/B_TDM_PlayerState Object Reference")))

(fn `GetTeamTotalKills`
  (params (TeamSide :type "EPlayableSide Enum" :default "Side_None"))
  (returns (`Total kills` :type Integer))
  (locals (TotalKills :type Integer) (NewLocalVar_0 :type "EPlayableSide Enum" :default "Side_None"))
  (switch `EPlayableSide` TeamSide
    (:`Side_None`
      _)
    (:`Side_Bluefor`
      (return (`self.BlueFor`)))
    (:`Side_Opfor`
      (return (`self.OpFor`)))
    (:`Side_Civ`
      _)
    (:`Side_AlwaysEnemy`
      _)
    (:`Side_Mercenary`
      _)
    (:`Side_Resistance`
      _))
  (return 0))

(fn `GetWinningTeam`
  (returns (`Winning Team` :type "EPlayableSide Enum"))
  (bind _total_kills (`self.GetTeamTotalKills` "Side_Bluefor"))
  (bind _total_kills_2 (`self.GetTeamTotalKills` "Side_Opfor"))
  (if (> _total_kills _total_kills_2)
    (return "Side_Bluefor")
    (elif (< _total_kills _total_kills_2)
      (return "Side_Opfor")
      (else
        (return "Side_None")))))

(fn `UserConstructionScript`)